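; Player controller that drives scene playback through a VisualController, stepping, fast-moving or auto-moving through scenes in both directions.
; The construction script creates the VisualController and applies the desktop resolution.
; BeginPlay adds the input mapping, configures preloading, sound, transitions and auto-move delay, then starts visualization with VisualRenderer.
; Enhanced Input actions forward navigation and cancel requests to the controller, or toggle BP_HUD visibility.
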(event `self.ReceiveBeginPlay`
  (bind _visualcontroller (`self.VisualController`))
  ;[1 0.288 0.2847] Check construction script for more on initialization
  (`EnhancedInputSubsystemInterface.AddMappingContext` (subsystem `EnhancedInputLocalPlayerSubsystem`) "/Game/Input/InputMappings/IMC_Game.IMC_Game" 0 (struct))
  ;[1 0.3124 0.7031] Configure visual controller here
  (`VisualController.SetNumScenesToLoad` _visualcontroller 5)
  (`VisualController.ShouldPlaySound` _visualcontroller true)
  (`VisualController.ShouldPlayTransitions` _visualcontroller true)
  (`VisualController.SetAutoMoveDelay` _visualcontroller 5.0)
  (`VisualController.Visualize` _visualcontroller "/Script/VisualU.VisualRenderer" 0)
  (`VisualController.Visualize` _visualcontroller "/Script/VisualU.VisualRenderer" 0))

(event `EnhancedInput|/Game/Input/InputActions/IA_Next`
  (params (ActionValue :type Boolean) (ElapsedSeconds :type "Float (double-precision)") (TriggeredSeconds :type "Float (double-precision)") (InputAction :type "InputAction Object Reference" :default "/Game/Input/InputActions/IA_Next.IA_Next"))
  ;[0.2829 1 0.5209] Input
  (:`Started`
    (`VisualController.RequestNextScene` (`self.VisualController`))))

(event `EnhancedInput|/Game/Input/InputActions/IA_CancelFastMove`
  (params (ActionValue :type Boolean) (ElapsedSeconds :type "Float (double-precision)") (TriggeredSeconds :type "Float (double-precision)") (InputAction :type "InputAction Object Reference" :default "/Game/Input/InputActions/IA_CancelFastMove.IA_CancelFastMove"))
  ;[0.2829 1 0.5209] Input
  (:`Started`
    (`VisualController.CancelFastMove` (`self.VisualController`))))

(event `EnhancedInput|/Game/Input/InputActions/IA_Previous`
  (params (ActionValue :type Boolean) (ElapsedSeconds :type "Float (double-precision)") (TriggeredSeconds :type "Float (double-precision)") (InputAction :type "InputAction Object Reference" :default "/Game/Input/InputActions/IA_Previous.IA_Previous"))
  ;[0.2829 1 0.5209] Input
  (:`Started`
    (`VisualController.RequestPreviousScene` (`self.VisualController`))))

(event `EnhancedInput|/Game/Input/InputActions/IA_CancelAutoMove`
  (params (ActionValue :type Boolean) (ElapsedSeconds :type "Float (double-precision)") (TriggeredSeconds :type "Float (double-precision)") (InputAction :type "InputAction Object Reference" :default "/Game/Input/InputActions/IA_CancelAutoMove.IA_CancelAutoMove"))
  ;[0.2829 1 0.5209] Input
  (:`Started`
    (`VisualController.CancelAutoMove` (`self.VisualController`))))

(event `EnhancedInput|/Game/Input/InputActions/IA_FastMove`
  (params (ActionValue :type Boolean) (ElapsedSeconds :type "Float (double-precision)") (TriggeredSeconds :type "Float (double-precision)") (InputAction :type "InputAction Object Reference" :default "/Game/Input/InputActions/IA_FastMove.IA_FastMove"))
  ;[0.2829 1 0.5209] Input
  (:`Started`
    (`VisualController.RequestFastMove` (`self.VisualController`) "Forward")))

(event `EnhancedInput|/Game/Input/InputActions/IA_HideHUD`
  (params (ActionValue :type Boolean) (ElapsedSeconds :type "Float (double-precision)") (TriggeredSeconds :type "Float (double-precision)") (InputAction :type "InputAction Object Reference" :default "/Game/Input/InputActions/IA_HideHUD.IA_HideHUD"))
  ;[0.2829 1 0.5209] Input
  (:`Started`
    (bind _asbp_hud (cast `/Game/Gameplay/BP_HUD` (`self.GetHUD`)))
    (`/Game/Gameplay/BP_HUD.ToggleHUD` _asbp_hud)))

(event `EnhancedInput|/Game/Input/InputActions/IA_ReverseFastMove`
  (params (ActionValue :type Boolean) (ElapsedSeconds :type "Float (double-precision)") (TriggeredSeconds :type "Float (double-precision)") (InputAction :type "InputAction Object Reference" :default "/Game/Input/InputActions/IA_ReverseFastMove.IA_ReverseFastMove"))
  ;[0.2829 1 0.5209] Input
  (:`Started`
    (`VisualController.RequestFastMove` (`self.VisualController`) "Backward")))

(event `EnhancedInput|/Game/Input/InputActions/IA_AutoMove`
  (params (ActionValue :type Boolean) (ElapsedSeconds :type "Float (double-precision)") (TriggeredSeconds :type "Float (double-precision)") (InputAction :type "InputAction Object Reference" :default "/Game/Input/InputActions/IA_AutoMove.IA_AutoMove"))
  ;[0.2829 1 0.5209] Input
  (:`Started`
    (`VisualController.RequestAutoMove` (`self.VisualController`) "Forward")))

(event `EnhancedInput|/Game/Input/InputActions/IA_ReverseAutoMove`
  (params (ActionValue :type Boolean) (ElapsedSeconds :type "Float (double-precision)") (TriggeredSeconds :type "Float (double-precision)") (InputAction :type "InputAction Object Reference" :default "/Game/Input/InputActions/IA_ReverseAutoMove.IA_ReverseAutoMove"))
  ;[0.2829 1 0.5209] Input
  (:`Started`
    (`VisualController.RequestAutoMove` (`self.VisualController`) "Backward")))

(fn `GetVisualController`
  (returns (ReturnValue :type "VisualController Object Reference"))
  (return (`self.VisualController`)))

(fn `UserConstructionScript`
  (`|ExecutionSequence`
    (:`then_0`
      (bind _returnvalue (`|GenericCreateObject` "/Script/VisualU.VisualController"))
      (set `self.VisualController` _returnvalue))
    (:`then_1`
      (bind _returnvalue_2 (`GameUserSettings.GetGameUserSettings`))
      (`GameUserSettings.SetScreenResolution` _returnvalue_2 (`GameUserSettings.GetDesktopResolution` _returnvalue_2))
      (`GameUserSettings.ApplyResolutionSettings` _returnvalue_2 false))))